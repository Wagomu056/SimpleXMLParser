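; Functional test Blueprint that verifies ParseXML output for a sample XML string.
; StartTest parses Contents, checks the element count against ExpectParsedDataNum, then validates the Title and Body keys and texts plus Body's id attribute.
; Check helpers call TestFail with a descriptive message on mismatch.
; Both TestFail and TestSuccess call QuitGame before FinishTest reports the result.
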(event EventStartTest
  (bind _parseddataarray (Class|SimpleXMLParserFunctionLibrary|ParseXML (Variables|Default|GetContents)))
  (bind _output_get (Variables|Default|SetParsed%20Data%20Array _parseddataarray))
  (if (== (Utilities|Array|Length _output_get) (Variables|Default|GetExpectParsedDataNum)) ; Check the number of parsed data.
    (Utilities|CheckParsedData (Utilities|Array|Get(acopy) (Variables|Default|GetParsed%20Data%20Array)) "Title" "Title Text" ; Check the first data.
      (:true
        (Utilities|CheckParsedData (Utilities|Array|Get(acopy) (Variables|Default|GetParsed%20Data%20Array) 1) "Body" "Body Text" ; Check the next data.
          (:true
            (|CheckAttribute (Utilities|Array|Get(acopy) (Variables|Default|GetParsed%20Data%20Array) 1)) ; Check the attribute.
            (Utilities|TestSuccess)))))
    (else
      (Utilities|TestFail (Utilities|GenerateTestFailMessage "The number of parsed data is invalid." (Utilities|String|ToString(Integer) (Variables|Default|GetExpectParsedDataNum)) (Utilities|String|ToString(Integer) (Utilities|Array|Length _output_get)))))))

(fn ConstructionScript)